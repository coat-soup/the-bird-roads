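; Nav agent component that paths a character relative to a Parent transform, using a static actor copy as the navigation space.
; FromWorld maps endpoints onto the copy for synchronous pathfinding; ToWorld maps points back to the Parent's current transform.
; Tick drives the character horizontally along the path with movement input and force, firing OnFinishedPath near the end.
; PathTick repaths to BP_Player, but its looping timer is disconnected.
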(event `self.ReceiveBeginPlay`
  (bind _returnvalue (`GameplayStatics.GetActorOfClass` "/Game/Player/Blueprints/BP_Player.BP_Player_C"))
  (set `self.Follow` _returnvalue))

(event `PathTick`
  (if (`self.IsComponentTickEnabled`)
    (`self.CalculatePathToWorldPosition` (`Actor.K2_GetActorLocation` (`self.Follow`)))))

(event `self.ReceiveTick`
  (params (DeltaSeconds :type "Float (single-precision)"))
  (if (`/Game/Characters/AI/AI_Character.Enabled` (`/Game/Characters/Blueprints/BP_Character.AIController` (`self.Character`)))
    (`/Engine/EditorBlueprintResources/StandardMacros.IsValid` (`self.Path`)
      (:`Is Valid`
        (`self.MoveToNextPathPoint`)
        (for (_array_element _array_index) (`NavigationPath.PathPoints` (`self.Path`))
          (bind _out (`self.ToWorld` _array_element)))))))

(event `MoveToNextPathPoint`
  (bind _character (`self.Character`))
  (bind _pathpoints (`NavigationPath.PathPoints` (`self.Path`)))
  (bind _returnvalue (- (`KismetArrayLibrary.Array_Length` (`NavigationPath.PathPoints` (`self.Path`))) 1))
  (bind _out (`self.ToWorld` (`|GetArrayItem` (`NavigationPath.PathPoints` (`self.Path`)) (`self.PathIndex`))))
  (`|ExecutionSequence`
    (:`then_0`
      (bind _returnvalue_2 (- _out (`Actor.K2_GetActorLocation` (`self.Character`))))
      (bind _returnvalue_3 (`KismetMathLibrary.VSize` _returnvalue_2))
      (if (< _returnvalue_3 100.0)
        (bind _output_get (set `self.PathIndex` (`KismetMathLibrary.Clamp` (+ (`self.PathIndex`) 1) 0 _returnvalue)))
        (if (>= _output_get _returnvalue)
          _)))
    (:`then_1`
      (bind _returnvalue_4 (* (* (/ _returnvalue_2 _returnvalue_3) (1.0 1.0 0.0)) 1.0))
      (`Pawn.AddMovementInput` _character _returnvalue_4 1.0 false)
      (`CharacterMovementComponent.AddForce` (`Character.CharacterMovement` _character) (* _returnvalue_4 1.0)))
    (:`then_2`
      (bind _out_2 (`self.ToWorld` (`|GetArrayItem` _pathpoints (`KismetArrayLibrary.Array_LastIndex` _pathpoints))))
      (if (<= (`KismetMathLibrary.Vector_Distance` _out_2 (`Actor.K2_GetActorLocation` (`self.Character`))) 150.0)
        (`self.OnFinishedPath`)))))

(event `CalculatePathToWorldPosition`
  (params (Position :type "Vector Structure"))
  (bind _returnvalue (`KismetArrayLibrary.Array_Length` (`NavigationPath.PathPoints` (`self.Path`))))
  (bind _out (`self.FromWorld` Position))
  (bind _out_2 (`self.FromWorld` (`Actor.K2_GetActorLocation` (`self.Character`))))
  (bind _returnvalue_2 (`NavigationSystemV1.FindPathToLocationSynchronously` _out_2 _out (`/Game/Characters/Blueprints/BP_Character.AIController` (`self.Character`)) null))
  (set `self.Path` _returnvalue_2)
  (set `self.PathIndex` 1)
  (if (<= _returnvalue 0)
    (`KismetSystemLibrary.PrintString` "No path found")
    (else
      (`KismetSystemLibrary.PrintString` "Pathing")
      (for _index (range 1 _returnvalue)
        (bind _out_3 (`self.ToWorld` (`|GetArrayItem` (`NavigationPath.PathPoints` (`self.Path`)) (`self.PathIndex`))))
        (if (<= (`KismetMathLibrary.Vector_Distance` _out_3 (`Actor.K2_GetActorLocation` (`self.Character`))) 150.0)
          (set `self.PathIndex` _index)
          (else
            (break)))))))

(fn `FromWorld`
  (params (In :type "Vector Structure"))
  (returns (Out :type "Vector Structure"))
  (return (`KismetMathLibrary.TransformLocation` (`Actor.GetTransform` (`self.StaticActorCopy`)) (`KismetMathLibrary.InverseTransformLocation` (`SceneComponent.K2_GetComponentToWorld` (`self.Parent`)) In))))

(fn `ToWorld`
  (params (In :type "Vector Structure"))
  (returns (Out :type "Vector Structure"))
  (return (`KismetMathLibrary.TransformLocation` (`SceneComponent.K2_GetComponentToWorld` (`self.Parent`)) (`KismetMathLibrary.InverseTransformLocation` (`Actor.GetTransform` (`self.StaticActorCopy`)) In))))